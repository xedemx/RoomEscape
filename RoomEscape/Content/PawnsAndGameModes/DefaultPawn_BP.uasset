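; Default player pawn that lets the player operate room doors and next-door buttons through the Interact input.
; On press, it line traces 500 units forward from the player camera manager against WorldStatic and WorldDynamic objects.
; The hit actor is cast directly rather than through an interface: a DoorToNextRoom gets OpenClose, otherwise a ButtonNextDoor gets Interact.
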(event Input|ActionEvents|InputActionInteract
  (params (Key :type Key%20Structure))
  (bind _returnvalue (Game|GetPlayerCameraManager 0))
  (bind _returnvalue_2 (Transformation|GetActorLocation _returnvalue))
  (:Pressed
    (bind (_outhit _returnvalue_3) (Collision|LineTraceForObjects _returnvalue_2 (+ _returnvalue_2 (* (Transformation|GetActorForwardVector _returnvalue) 5e+02)) (Utilities|Array|MakeArray "ObjectTypeQuery1" "ObjectTypeQuery2") false 0 "None"))
    (if _returnvalue_3
      (bind _asdoor_to_next_room (Utilities|Casting|CastToDoorToNextRoom (.HitActor (Collision|BreakHitResult _outhit)))
        (:then
          (Default|Open/Close _asdoor_to_next_room))
        (:CastFailed
          (bind _asbutton_next_door (Utilities|Casting|CastToButtonNextDoor (.HitActor (Collision|BreakHitResult _outhit))))
          (Default|Interact _asbutton_next_door))))))

(fn ConstructionScript)